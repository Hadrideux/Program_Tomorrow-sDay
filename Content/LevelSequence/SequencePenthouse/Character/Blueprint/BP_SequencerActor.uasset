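; Sequencer character actor for the penthouse sequence, with a skeletal mesh, audio and decal that react to the active camera filter.
; Once the scene manager initializes, it caches the sequencer and camera managers, and sequence play or stop unpauses or pauses audio.
; Tick polls the filter: thermal enables custom depth on the mesh, while audio unmutes sound and shows the decal only during playback.
; Any audio play-state change re-mutes the sound.
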(event OnAudioPlayStateChanged(Audio)
  (params (PlayState :type EAudioComponentPlayState%20Enum :default "Playing"))
  (switch Utilities|FlowControl|Switch|SwitchonEAudioComponentPlayState PlayState
    (:Playing
      _)
    (:Stopped
      _)
    (:Paused
      _))
  (CallFunction|MuteAudio))

(event Custom|OnPlaySequence_Event
  (params (SequencerState :type ESequencerState%20Enum :default "NewEnumerator0"))
  (switch Utilities|FlowControl|Switch|SwitchonESequencerState SequencerState
    (:NewEnumerator1
      (CallFunction|UnpauseAudio))
    (:NewEnumerator2
      (CallFunction|PauseAudio))))

(event Custom|BindInit
  ;[1 1 1] Initialization Binding Event
  (bind _output_get (Variables|Default|SetScene%20Manager (.AsBP%20Scene%20Manager (Utilities|Casting|CastToBP_SceneManager (CallFunction|GetSingletonInstance "/Game/Blueprint/Global/Manager/BP_SceneManager.BP_SceneManager_C")))))
  (EventDispatchers|BindEventtoOnInitiateManagerEvent _output_get (delegate Custom|BindInitEvent)))

(event Custom|ThermalRender
  (params (bValue :type Boolean))
  ;[1 1 1] Set Visibility Decal Filter
  (Rendering|SetRenderCustomDepth (Variables|Default|GetSkeletalMesh) bValue))

(event Custom|BindSequenceControl
  (EventDispatchers|BindEventtoOnSequenceStateChange (Variables|Default|GetSequencer%20Manager) (delegate Custom|OnPlaySequence_Event)))

(event Custom|BindInitEvent
  ;[1 1 1] Initialization Binding Event
  (Utilities|FlowControl|Sequence
    (:then_0
      (CallFunction|SetManagerVariable))
    (:then_1
      (CallFunction|BindAllEvent))))

(event Custom|PlayAudio
  (params (NewSound :type Sound%20Base%20Object%20Reference))
  (bind _audio (Variables|Default|GetAudio))
  ;[1 1 1] Set Audio Play and Volume
  (if (not (Audio|Components|Audio|IsPlaying _audio))
    (Audio|Components|Audio|SetSound _audio NewSound)
    (Audio|Components|Audio|Play _audio 0.0)))

(event Custom|StopAudio
  ;[1 1 1] Set Audio Play and Volume
  (Audio|Components|Audio|Stop (Variables|Default|GetAudio)))

(event Custom|HiddeDecal
  ;[1 1 1] Set Visibility Decal Filter
  (Rendering|SetVisibility (Variables|Default|GetDecal) false false))

(event Custom|VisibleDecal
  ;[1 1 1] Set Visibility Decal Filter
  (Rendering|SetVisibility (Variables|Default|GetDecal) true false))

(event EventBeginPlay
  ;[1 1 1] Initialization Binding Event
  (CallFunction|BindInit))

(event EventTick
  (params (DeltaSeconds :type Float%20%28single-precision%29))
  (bind _scene_manager (Variables|Default|GetScene%20Manager))
  (bind _cameraactormanager (Variables|/Game/Blueprint/Global/Manager/BP_SceneManager.BP_SceneManager_C|GetCameraActorManager _scene_manager))
  (Utilities|IsValid _cameraactormanager
    (:Is%20Valid
      (switch Utilities|FlowControl|Switch|SwitchonECameraFilter (Variables|/Game/Blueprint/Global/Manager/BP_CameraActorManager.BP_CameraActorManager_C|GetECurrentCameraFilter _cameraactormanager)
        (:NewEnumerator0
          (CallFunction|MuteAudio :!label _label)
          (CallFunction|HiddeDecal :!label _label_2)
          (CallFunction|ThermalRender false :!label _label_3))
        (:NewEnumerator1
          (goto _label))
        (:NewEnumerator2
          (CallFunction|MuteAudio)
          (CallFunction|HiddeDecal)
          (CallFunction|ThermalRender true))
        (:NewEnumerator3
          (CallFunction|UnmuteAudio)
          (switch Utilities|FlowControl|Switch|SwitchonEAudioComponentPlayState (Audio|Components|Audio|GetPlayState (Variables|Default|GetAudio))
            (:Playing
              (CallFunction|VisibleDecal)
              (goto _label_3))
            (:Stopped
              (goto _label_2))
            (:Paused
              (goto _label_2))))))))

(fn ConstructionScript)

(fn BindAllEvent
  (CallFunction|BindSequenceControl))

(fn SetManagerVariable
  (bind _scene_manager (Variables|Default|GetScene%20Manager))
  (Variables|Default|SetSequencer%20Manager (Variables|/Game/Blueprint/Global/Manager/BP_SceneManager.BP_SceneManager_C|GetSequencerManager _scene_manager))
  (Variables|Default|SetCamera%20Manager (Variables|/Game/Blueprint/Global/Manager/BP_SceneManager.BP_SceneManager_C|GetCameraActorManager _scene_manager)))