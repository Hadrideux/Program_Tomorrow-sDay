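; Hint actor that configures its visual from its hint type: UV, thermal, audio or citizen.
; The construction script shows a cube for UV, thermal and audio hints, and a skeletal mesh for citizens.
; Thermal and citizen hints set custom depth rendering and a stencil value on the shown mesh.
; Manager references are cached from SceneManager, while event binding and filter visibility functions are empty stubs.
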(fn ConstructionScript
  (bind _skeletalmesh (Variables|Default|GetSkeletalMesh))
  (bind _cube (Variables|Default|GetCube))
  (switch Utilities|FlowControl|Switch|SwitchonEHintType (Variables|HintType|GetEHintType)
    (:NewEnumerator1
      (Rendering|SetVisibility (Variables|Default|GetCube) true false :!label _label)
      (Rendering|SetVisibility (Variables|Default|GetSkeletalMesh) false false))
    (:NewEnumerator2
      (Rendering|SetRenderCustomDepth _cube (Variables|ThermalFilter|GetThermalRender))
      (Rendering|SetCustomDepthStencilValue _cube (Variables|ThermalFilter|GetThermalStencilValue))
      (goto _label))
    (:NewEnumerator3
      (goto _label))
    (:NewEnumerator4
      (Rendering|SetVisibility (Variables|Default|GetSkeletalMesh) true false)
      (Rendering|SetRenderCustomDepth _skeletalmesh (Variables|ThermalFilter|GetThermalRender))
      (Rendering|SetCustomDepthStencilValue _skeletalmesh (Variables|ThermalFilter|GetThermalStencilValue))
      (Rendering|SetVisibility (Variables|Default|GetCube) false false))))

(fn SetManagerVariable
  (bind _scene_manager (Variables|Manager|GetScene%20Manager))
  (Variables|Manager|SetGame%20State%20Manager (Variables|/Game/Blueprint/Global/Manager/BP_SceneManager.BP_SceneManager_C|GetGameStateManager _scene_manager))
  (Variables|Manager|SetHint%20Manager (Variables|/Game/Blueprint/Global/Manager/BP_SceneManager.BP_SceneManager_C|GetHintManager _scene_manager))
  (Variables|Manager|SetSequencer%20Manager (Variables|/Game/Blueprint/Global/Manager/BP_SceneManager.BP_SceneManager_C|GetSequencerManager _scene_manager))
  (Variables|Manager|SetCamera%20Actor%20Manager (Variables|/Game/Blueprint/Global/Manager/BP_SceneManager.BP_SceneManager_C|GetCameraActorManager _scene_manager)))

(fn BindAllEvent)

(fn SetVisibilityFIlter
  (params (Set%20Visibility :type Boolean)))