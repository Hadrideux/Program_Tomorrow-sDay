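; BP_AudioHintController is an audio hint actor with a citizen skeletal mesh, whose sound HintManager events can mute or unmute.
; After the SceneManager's initiate event, it sets its manager variable and binds to HintManager's volume-change and active-filter events.
; Volume changes apply only when the event targets this instance, setting the Audio component's volume multiplier.
; The active-filter handler switches on the filter value but performs no actions.
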(event Custom|BindAudioVolume
  (EventDispatchers|AssignOnChangeAudioVolume (Variables|Default|GetHint%20Manager) (delegate Custom|ChangeVolume_Event)))

(event Custom|ChangeVolume_Event
  (params (EAudio%20Volume :type EAudioVolumeState%20Enum :default "NewEnumerator0") (Audio%20Hint%20Changed :type BP%20Audio%20Hint%20Controller%20Object%20Reference))
  (if (== Audio%20Hint%20Changed self)
    (switch Utilities|FlowControl|Switch|SwitchonEAudioVolumeState EAudio%20Volume
      (:NewEnumerator1
        (CallFunction|AudioVolume 0.0))
      (:NewEnumerator2
        (CallFunction|AudioVolume 1.0)))))

(event Custom|Initialization_Event
  ;[1 1 1] Initialization Binding Event
  (Utilities|FlowControl|Sequence
    (:then_0
      (CallFunction|SetManagerVariable))
    (:then_1
      (CallFunction|BindAllEvent))))

(event Custom|BindActiveFilter
  (EventDispatchers|AssignOnActiveFilterVisual (Variables|Default|GetHint%20Manager) (delegate Custom|ActiveFilter_Event)))

(event Custom|ActiveFilter_Event
  (params (EActiveFilter :type ECameraFilter%20Enum :default "NewEnumerator0"))
  (switch Utilities|FlowControl|Switch|SwitchonECameraFilter EActiveFilter))

(event EventBeginPlay
  ;[1 1 1] Initialization Binding Event
  (bind _output_get (Variables|Default|SetScene%20Manager (CallFunction|InitiateSceneManager)))
  (EventDispatchers|BindEventtoOnInitiateManagerEvent _output_get (delegate Custom|Initialization_Event)))

(fn ConstructionScript
  (|CallParentFunction)
  (Components|SkeletalMesh|SetSkeletalMeshAsset (Variables|Default|GetSkeletalMesh) (Variables|Default|GetSkeletal%20Citizen)))

(fn BindAllEvent
  (CallFunction|BindAudioVolume)
  (CallFunction|BindActiveFilter))

(fn AudioVolume
  (params (VolumeMultiplier :type Float%20%28single-precision%29))
  (Audio|Components|Audio|SetVolumeMultiplier (Variables|Default|GetAudio) VolumeMultiplier :!class /Script/Engine.AudioComponent))