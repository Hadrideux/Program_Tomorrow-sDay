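; Actor component that stores the analysis state and information of an investigation hint.
; It waits for the BP_SceneManager singleton's initialization, then caches the investigation and camera managers and binds to analysis events.
; Progress events update the hint element, UV hint and image, and completion sets the analysis index, each only when this component is the current hint.
; A helper function shows one decal and hides a list of others.
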(event Custom|BindAnalyseBreak
  ;[1 1 1] Added Hint Information
  (EventDispatchers|BindEventtoOnAnalyseComplete (Variables|Manager|GetInvestigation%20Manager) (delegate Custom|AnalyseBreak%20Event)))

(event Custom|BindInit
  ;[1 1 1] Initialization Binding Event
  (bind _output_get (Variables|Manager|SetScene%20Manager (.AsBP%20Scene%20Manager (Utilities|Casting|CastToBP_SceneManager (CallFunction|GetSingletonInstance "/Game/Blueprint/Global/Manager/BP_SceneManager.BP_SceneManager_C")))))
  (EventDispatchers|BindEventtoOnInitializationBind _output_get (delegate Custom|Init%20Event)))

(event Custom|Init%20Event
  ;[1 1 1] Initialization Binding Event
  (Utilities|FlowControl|Sequence
    (:then_0
      (CallFunction|SetManagerVariable))
    (:then_1
      (CallFunction|BindAllEvent))))

(event Custom|AnalyseBreak%20Event
  (params (CurrentHint :type AC%20Hint%20Information%20Object%20Reference) (Analyse%20Index :type Integer))
  ;[1 1 1] Added Hint Information
  (if (== CurrentHint self)
    (Variables|Analysis|SetCurrentAnalyseIndex Analyse%20Index)))

(event Custom|BindAnallyseInProgress
  ;[1 1 1] Added Hint Information
  (EventDispatchers|BindEventtoOnAnalyseinProgress (Variables|Manager|GetInvestigation%20Manager) (delegate Custom|AnalyseInProgress%20Event)))

(event Custom|AnalyseInProgress%20Event
  (params (CurrentHint :type AC%20Hint%20Information%20Object%20Reference) (HintElement :type S%20Hint%20Structure) (UVHint :type S%20Hint%20UV%20Info%20Structure) (Image :type Texture%202D%20Object%20Reference))
  ;[1 1 1] Added Hint Information
  (if (== CurrentHint self)
    (Variables|Analysis|SetHint%20Information HintElement)
    (Variables|Analysis|SetUVHintInformation UVHint)
    (Variables|Analysis|SetHintImage Image)))

(event EventBeginPlay
  ;[1 1 1] Initialization Binding Event
  (CallFunction|BindInit))

(fn BindAllEvent
  (CallFunction|BindAnalyseBreak)
  (CallFunction|BindAnallyseinProgress))

(fn SetManagerVariable
  (bind _scene_manager (Variables|Manager|GetScene%20Manager))
  (Variables|Manager|SetInvestigation%20Manager (Variables|/Game/Blueprint/Global/Manager/BP_SceneManager.BP_SceneManager_C|GetInvestigation%20Manager _scene_manager))
  (Variables|Manager|SetCamera%20Manager (Variables|/Game/Blueprint/Global/Manager/BP_SceneManager.BP_SceneManager_C|GetCameraManager _scene_manager)))

(fn EnableandDisableDecal
  (params (ActiveDecal :type Decal%20Actor%20Object%20Reference) (DeactiveDecal :type Array%20of%20Decal%20Actor%20Object%20References))
  (Utilities|IsValid ActiveDecal
    (:Is%20Valid
      (Utilities|FlowControl|Sequence
        (:then_0
          (Rendering|SetVisibility (Variables|/Script/Engine.DecalActor|GetDecal ActiveDecal) true false))
        (:then_1
          (for _array_element DeactiveDecal :!label _label
            (Utilities|IsValid _array_element
              (:Is%20Valid
                (Rendering|SetVisibility (Variables|/Script/Engine.Actor|GetRootComponent _array_element) false false)))))))
    (:Is%20Not%20Valid
      (goto _label))))