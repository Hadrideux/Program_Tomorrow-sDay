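; UV hint controller that activates its Decal component for the UV filter and deactivates it for the thermal and audio filters.
; On BeginPlay it waits for the scene manager's initiate-manager event, then sets manager variables and calls BindAllEvent.
; A separate BindActiveFilter event subscribes to HintManager's filter-visual event to drive the toggle.
; BindAllEvent is empty, and nothing in this Blueprint calls BindActiveFilter.
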(event Custom|Initialization_Event
  ;[1 1 1] Initialization Binding Event
  (Utilities|FlowControl|Sequence
    (:then_0
      (CallFunction|SetManagerVariable))
    (:then_1
      (CallFunction|BindAllEvent))))

(event Custom|BindActiveFilter
  (EventDispatchers|AssignOnActiveFilterVisual (Variables|Default|GetHint%20Manager) (delegate Custom|ActiveFilter_Event)))

(event Custom|ActiveFilter_Event
  (params (EActiveFilter :type ECameraFilter%20Enum :default "NewEnumerator0"))
  (switch Utilities|FlowControl|Switch|SwitchonECameraFilter EActiveFilter
    (:NewEnumerator1
      (CallFunction|ActiveFilter true))
    (:NewEnumerator2
      (CallFunction|ActiveFilter false :!label _label))
    (:NewEnumerator3
      (goto _label))))

(event EventBeginPlay
  ;[1 1 1] Initialization Binding Event
  (bind _output_get (Variables|Default|SetScene%20Manager (CallFunction|InitiateSceneManager)))
  (EventDispatchers|BindEventtoOnInitiateManagerEvent _output_get (delegate Custom|Initialization_Event)))

(fn ConstructionScript
  (|CallParentFunction))

(fn BindAllEvent)

(fn ActiveFilter
  (params (bNewActive :type Boolean))
  (Components|Activation|SetActive (Variables|Default|GetDecal) bNewActive false))