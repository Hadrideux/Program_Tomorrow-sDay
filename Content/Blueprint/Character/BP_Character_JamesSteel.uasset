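; James Steel's playable character: a fixed-viewpoint first-person camera for looking around, highlighting and selecting desk elements and faxes.
; After scene manager initialization, it registers with the player controller and binds look and selection, with view angles clamped around the camera's facing.
; Looking line-traces to toggle custom-depth highlights and an input hint widget.
; Selection possesses a clicked pawn or starts a fax investigation; a timeline drives FOV zoom.
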(event Custom|OnLookAround
  (params (ActionValue :type Vector%202D%20Structure))
  ;[1 1 1] LookAt and Focus
  (CallFunction|LookAround ActionValue)
  (CallFunction|Focus))

(event Custom|BindLookAround
  ;[1 1 1] LookAt and Focus
  (EventDispatchers|AssignOnLookAround (Variables|Manager|GetPlayerController) (delegate Custom|OnLookAround)))

(event Custom|BindSelection
  ;[1 1 1] PlayerSelection
  (EventDispatchers|AssignOnSelection (Variables|Manager|GetPlayerController) (delegate Custom|OnSelection)))

(event Custom|OnSelection
  ;[1 1 1] PlayerSelection
  (bind _hitactor (CallFunction|ObjectClicked "TraceTypeQuery3"))
  (bind _aspawn (Utilities|Casting|CastToPawn _hitactor)
    (:then
      (Default|CallOnNewPossessPawn (Variables|Manager|GetPlayerController) _aspawn))
    (:CastFailed
      (bind _asbp_fax (Utilities|Casting|CastToBP_Fax _hitactor))
      (Default|StartNewInvestigation _asbp_fax)
      (Rendering|SetRenderCustomDepth (Variables|/Game/Blueprint/Office/BP_Fax.BP_Fax_C|GetFax _asbp_fax) true)))
  (if (UserInterface|Viewport|IsinViewport (Variables|Default|GetWBP_InputIndication))
    (Widget|RemovefromParent (Variables|Default|GetWBP_InputIndication))))

(event Custom|BindInit
  ;[1 1 1] Initialization
  (bind _output_get (Variables|Manager|SetScene%20Manager (.AsBP%20Scene%20Manager (Utilities|Casting|CastToBP_SceneManager (CallFunction|GetSingletonInstance "/Game/Blueprint/Global/Manager/BP_SceneManager.BP_SceneManager_C")))))
  (EventDispatchers|BindEventtoOnInitializationBind _output_get (delegate Custom|Initiate_Event)))

(event Custom|Initiate_Event
  (bind _playercontroller (Variables|Manager|GetPlayerController))
  ;[1 1 1] Initialization
  (Utilities|FlowControl|Sequence
    (:then_0
      (CallFunction|SetManagerVariable)
      (CallFunction|Contraint)
      (bind _output_get (Variables|/Game/Blueprint/Global/BP_TomorrowsDay_PC.BP_TomorrowsDay_PC_C|SetJamesSteel _playercontroller self))
      (Variables|/Game/Blueprint/Global/BP_TomorrowsDay_PC.BP_TomorrowsDay_PC_C|SetCurrentPossess _playercontroller _output_get))
    (:then_1
      (CallFunction|BindAllEvent)
      (bind _returnvalue (UserInterface|CreateWidget "/Game/Widget/FeedBack/WBP_InputIndication.WBP_InputIndication_C"))
      (Variables|Default|SetWBP_InputIndication _returnvalue))))

(event Input|EnhancedActionEvents|EnhancedInputActionIA_Zoom
  (params (ActionValue :type Boolean) (ElapsedSeconds :type Float%20%28double-precision%29) (TriggeredSeconds :type Float%20%28double-precision%29) (InputAction :type Input%20Action%20Object%20Reference :default "/Game/Blueprint/Character/Input/Action/Game/IA_Zoom.IA_Zoom"))
  ;[1 1 1] Zoom
  (:Started
    (bind _zoom (Timeline|Zoom Play)
      (:Update
        (Camera|SetFieldOfView (Variables|Default|GetCamera) (Math|Float|Lerp 9e+01 45.0 _zoom)))))
  (:Completed
    (Timeline|Zoom Reverse)))

(event EventBeginPlay
  ;[1 1 1] Initialization
  (CallFunction|BindInit))

(fn ConstructionScript
  (CallFunction|Contraint))

(fn LookAround
  (params (InputAxis :type Vector%202D%20Structure))
  (Pawn|Input|AddControllerYawInput (.x InputAxis))
  (Pawn|Input|AddControllerPitchInput (.y InputAxis)))

(fn Contraint
  (bind _returnvalue (Game|GetPlayerCameraManager 0))
  (bind _camera (Variables|Default|GetCamera))
  (bind _camera_2 (Variables|Default|GetCamera))
  (bind _returnvalue_2 (Transformation|GetWorldRotation _camera))
  (bind _returnvalue_3 (Transformation|GetWorldRotation _camera_2))
  (Utilities|FlowControl|Sequence
    (:then_0
      (Variables|/Script/Engine.PlayerCameraManager|SetViewPitchMax _returnvalue (+ (Variables|ContraintView|GetPitchValue) (.pitch _returnvalue_3)))
      (Variables|/Script/Engine.PlayerCameraManager|SetViewYawMax _returnvalue (+ (Variables|ContraintView|GetYawValue) (.yaw _returnvalue_3))))
    (:then_1
      (Variables|/Script/Engine.PlayerCameraManager|SetViewPitchMin _returnvalue (- (.pitch _returnvalue_2) (Variables|ContraintView|GetPitchValue)))
      (Variables|/Script/Engine.PlayerCameraManager|SetViewYawMin _returnvalue (- (.yaw _returnvalue_2) (Variables|ContraintView|GetYawValue))))))

(fn ObjectClicked
  (params (TraceChannel :type ETraceTypeQuery%20Enum :default "TraceTypeQuery1"))
  (bind _camera (Variables|Default|GetCamera))
  (bind _returnvalue (Transformation|GetWorldLocation _camera))
  (bind _outhit (Collision|LineTraceByChannel _returnvalue (+ _returnvalue (* (Math|Vector|GetForwardVector (Transformation|GetWorldRotation (Variables|Default|GetCamera))) 1e+03)) TraceChannel true 0 "None"))
  (return (.HitActor (Collision|BreakHitResult _outhit))))

(fn SetManagerVariable
  (params (Scene%20Manager :type BP%20Scene%20Manager%20Object%20Reference))
  (Variables|Manager|SetPlayerController (.AsBP%20Tomorrows%20Day%20PC (Utilities|Casting|CastToBP_TomorrowsDay_PC (Game|GetPlayerController 0)))))

(fn BindAllEvent
  (CallFunction|BindLookAround)
  (CallFunction|BindSelection))

(fn Focus
  (Utilities|FlowControl|Sequence
    (:then_0
      (Utilities|IsValid (Variables|Default|GetCurrent%20Desk%20Element%20Focused)
        (:Is%20Valid
          (Rendering|SetRenderCustomDepth (Variables|/Game/Blueprint/Office/BP_DeskElement.BP_DeskElement_C|GetStaticMesh (Variables|Default|GetCurrent%20Desk%20Element%20Focused)) false))
        (:Is%20Not%20Valid
          _))
      (bind _hitactor (CallFunction|ObjectClicked (Variables|Default|GetTrace%20Channel)))
      (bind _asbp_desk_element (Utilities|Casting|CastToBP_DeskElement _hitactor)
        (:then
          (Rendering|SetRenderCustomDepth (Variables|/Game/Blueprint/Office/BP_DeskElement.BP_DeskElement_C|GetStaticMesh _asbp_desk_element) true)
          (Variables|Default|SetCurrent%20Desk%20Element%20Focused _asbp_desk_element)
          (if (not (UserInterface|Viewport|IsinViewport (Variables|Default|GetWBP_InputIndication))) :!label _label
            (UserInterface|Viewport|AddtoViewport (Variables|Default|GetWBP_InputIndication) 1)))
        (:CastFailed
          (if (UserInterface|Viewport|IsinViewport (Variables|Default|GetWBP_InputIndication))
            (Widget|RemovefromParent (Variables|Default|GetWBP_InputIndication))))))
    (:then_1
      (Utilities|IsValid (Variables|Default|GetFocusFax)
        (:Is%20Valid
          (Rendering|SetRenderCustomDepth (Variables|/Game/Blueprint/Office/BP_Fax.BP_Fax_C|GetFax (Variables|Default|GetFocusFax)) false))
        (:Is%20Not%20Valid
          _))
      (bind _hitactor_2 (CallFunction|ObjectClicked (Variables|Default|GetTrace%20Channel)))
      (bind _asbp_fax (Utilities|Casting|CastToBP_Fax _hitactor_2))
      (Rendering|SetRenderCustomDepth (Variables|/Game/Blueprint/Office/BP_Fax.BP_Fax_C|GetFax _asbp_fax) true)
      (Variables|Default|SetFocusFax _asbp_fax)
      (goto _label))))