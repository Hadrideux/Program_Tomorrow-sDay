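; Controller for the Data Center citizen search, linking the HUB screen widget to the data, UI and investigation managers.
; After SceneManager's initialization event, it caches those references and binds their events.
; Committed search text is substring-matched, ignoring case, against each citizen row's flattened fields, firing a DataManager result-entry event per matching field.
; Result clicks trigger research display; new-investigation events start the hardcoded "PowelsFamilly" row's investigation.
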(event Custom|Search
  (params (GetRecherche :type Text))
  (bind _data_manager (Variables|Manager|GetData%20Manager))
  (bind _citizendata (Variables|/Game/Blueprint/Global/Manager/BP_DataManager.BP_DataManager_C|GetCitizenData _data_manager))
  ;[1 1 1] Research in Data
  (bind _outrownames (DataTable|GetDataTableRowNames _citizendata))
  (bind _array_element (Utilities|Array|ForEachLoopwithBreak _outrownames)
    (:LoopBody
      (bind _array (Get|GetCitizenData _citizendata _array_element))
      (bind _array_element_2 (Utilities|Array|ForEachLoopwithBreak _array)
        (:LoopBody
          (bind _searchcontains (CallFunction|SearchExistinData _array_element_2 GetRecherche))
          (if _searchcontains
            (CallFunction|AddSearchResultEntry _array_element)))))))

(event Custom|AddSearchResultEntry
  (params (RowName :type Name))
  ;[1 1 1] Add Result Button
  (Default|CallOnAddSearchEntry (Variables|Manager|GetData%20Manager) RowName))

(event Custom|BindInit
  ;[1 1 1] Initialization Binding Event
  (bind _output_get (Variables|Manager|SetSceneManager (.AsBP%20Scene%20Manager (Utilities|Casting|CastToBP_SceneManager (CallFunction|GetSingletonInstance "/Game/Blueprint/Global/Manager/BP_SceneManager.BP_SceneManager_C")))))
  (EventDispatchers|BindEventtoOnInitializationBind _output_get (delegate Custom|BindInitEvent))
  (Variables|Manager|SetTomorrows%20Day%20PC (.AsBP%20Tomorrows%20Day%20PC (Utilities|Casting|CastToBP_TomorrowsDay_PC (Game|GetPlayerController 0)))))

(event Custom|BindInitEvent
  ;[1 1 1] Initialization Binding Event
  (Utilities|FlowControl|Sequence
    (:then_0
      (CallFunction|SetMaangerVariable))
    (:then_1
      (CallFunction|BindAllEvent))))

(event Custom|AddnewInvestigation
  (bind _returnvalue (Utilities|GetDataTableRow "/Game/DataBase/DT_Investigation.DT_Investigation" "PowelsFamilly")
    (:then
      (Default|CallOnStartInvestigation (Variables|Manager|GetInvestigation%20Manager) (.Order (Utilities|Struct|BreakSInvestigation _returnvalue))))))

(event Custom|BindNewInvestigation
  (EventDispatchers|BindEventtoOnNewInvestigation (Variables|Manager|GetInvestigation%20Manager) (delegate Custom|AddnewInvestigation)))

(event Custom|TextCommitted
  (params (Text :type Text%20%28by%20ref%29) (CommitMethod :type ETextCommit%20Enum :default "Default"))
  (bind _datacenterwidget (Variables|Widget|GetDataCenterWidget))
  (bind _researchbarbox (Variables|/Game/Widget/HUBScreen/InformationsCenter/WBP_InformationsCenter.WBP_InformationsCenter_C|GetResearchBarBox _datacenterwidget))
  ;[1 1 1] Get Research
  (switch Utilities|FlowControl|Switch|SwitchonETextCommit CommitMethod
    (:OnEnter
      (CallFunction|Search Text))
    (:OnCleared
      (Variables|/Script/UMG.EditableText|SetText _researchbarbox "")
      (Variables|/Script/UMG.EditableText|SetHintText _researchbarbox "Click here to search"))))

(event Custom|BindReseacrchBar
  ;[1 1 1] Get Research
  (EventDispatchers|AssignOnTextCommitted (Variables|/Game/Widget/HUBScreen/InformationsCenter/WBP_InformationsCenter.WBP_InformationsCenter_C|GetResearchBarBox (Variables|Widget|GetDataCenterWidget)) (delegate Custom|TextCommitted)))

(event Custom|DisplayDataButtonSearch
  (params (RowName :type Name))
  ;[1 1 1] Display Research
  (Default|CallOnDisplayResearch (Variables|Manager|GetData%20Manager) RowName))

(event Custom|BindButtonSearch
  ;[1 1 1] Display Research
  (EventDispatchers|BindEventtoOnClickSearchButton (Variables|Manager|GetUIManager) (delegate Custom|DisplayDataButtonSearch)))

(event EventBeginPlay
  ;[1 1 1] Initialization Binding Event
  (CallFunction|BindInit))

(fn ConstructionScript)

(fn GetCitizenData
  (params (DataTable :type Data%20Table%20Object%20Reference) (RowName :type Name))
  (bind _returnvalue (Utilities|GetDataTableRow DataTable RowName)
    (:then
      (Utilities|Array|AppendArray (Utilities|Array|MakeArray (.Work (Utilities|Struct|BreakSPersonalCitizenInfo (.PersonnalInfo (Utilities|Struct|BreakSCitizen _returnvalue)))) (.Activity (Utilities|Struct|BreakSPersonalCitizenInfo (.PersonnalInfo (Utilities|Struct|BreakSCitizen _returnvalue)))) (.Habits (Utilities|Struct|BreakSPersonalCitizenInfo (.PersonnalInfo (Utilities|Struct|BreakSCitizen _returnvalue)))) (.IdentityNumber (Utilities|Struct|BreakSOfficialCitizenInfo (.OfficialInfo (Utilities|Struct|BreakSCitizen _returnvalue)))) (.Name (Utilities|Struct|BreakSOfficialCitizenInfo (.OfficialInfo (Utilities|Struct|BreakSCitizen _returnvalue)))) (.FirstName (Utilities|Struct|BreakSOfficialCitizenInfo (.OfficialInfo (Utilities|Struct|BreakSCitizen _returnvalue)))) (.BirthPlace (Utilities|Struct|BreakSOfficialCitizenInfo (.OfficialInfo (Utilities|Struct|BreakSCitizen _returnvalue)))) (.Birthdate (Utilities|Struct|BreakSOfficialCitizenInfo (.OfficialInfo (Utilities|Struct|BreakSCitizen _returnvalue)))) (.Adress (Utilities|Struct|BreakSOfficialCitizenInfo (.OfficialInfo (Utilities|Struct|BreakSCitizen _returnvalue)))) (.Sexe (Utilities|Struct|BreakSOfficialCitizenInfo (.OfficialInfo (Utilities|Struct|BreakSCitizen _returnvalue)))) (.Height (Utilities|Struct|BreakSOfficialCitizenInfo (.OfficialInfo (Utilities|Struct|BreakSCitizen _returnvalue))))) (.Relation (Utilities|Struct|BreakSPersonalCitizenInfo (.PersonnalInfo (Utilities|Struct|BreakSCitizen _returnvalue)))))
      (Utilities|Array|AppendArray (Utilities|Array|MakeArray (.Work (Utilities|Struct|BreakSPersonalCitizenInfo (.PersonnalInfo (Utilities|Struct|BreakSCitizen _returnvalue)))) (.Activity (Utilities|Struct|BreakSPersonalCitizenInfo (.PersonnalInfo (Utilities|Struct|BreakSCitizen _returnvalue)))) (.Habits (Utilities|Struct|BreakSPersonalCitizenInfo (.PersonnalInfo (Utilities|Struct|BreakSCitizen _returnvalue)))) (.IdentityNumber (Utilities|Struct|BreakSOfficialCitizenInfo (.OfficialInfo (Utilities|Struct|BreakSCitizen _returnvalue)))) (.Name (Utilities|Struct|BreakSOfficialCitizenInfo (.OfficialInfo (Utilities|Struct|BreakSCitizen _returnvalue)))) (.FirstName (Utilities|Struct|BreakSOfficialCitizenInfo (.OfficialInfo (Utilities|Struct|BreakSCitizen _returnvalue)))) (.BirthPlace (Utilities|Struct|BreakSOfficialCitizenInfo (.OfficialInfo (Utilities|Struct|BreakSCitizen _returnvalue)))) (.Birthdate (Utilities|Struct|BreakSOfficialCitizenInfo (.OfficialInfo (Utilities|Struct|BreakSCitizen _returnvalue)))) (.Adress (Utilities|Struct|BreakSOfficialCitizenInfo (.OfficialInfo (Utilities|Struct|BreakSCitizen _returnvalue)))) (.Sexe (Utilities|Struct|BreakSOfficialCitizenInfo (.OfficialInfo (Utilities|Struct|BreakSCitizen _returnvalue)))) (.Height (Utilities|Struct|BreakSOfficialCitizenInfo (.OfficialInfo (Utilities|Struct|BreakSCitizen _returnvalue))))) (.Family (Utilities|Struct|BreakSPersonalCitizenInfo (.PersonnalInfo (Utilities|Struct|BreakSCitizen _returnvalue)))))
      (return (Utilities|Array|MakeArray (.Work (Utilities|Struct|BreakSPersonalCitizenInfo (.PersonnalInfo (Utilities|Struct|BreakSCitizen _returnvalue)))) (.Activity (Utilities|Struct|BreakSPersonalCitizenInfo (.PersonnalInfo (Utilities|Struct|BreakSCitizen _returnvalue)))) (.Habits (Utilities|Struct|BreakSPersonalCitizenInfo (.PersonnalInfo (Utilities|Struct|BreakSCitizen _returnvalue)))) (.IdentityNumber (Utilities|Struct|BreakSOfficialCitizenInfo (.OfficialInfo (Utilities|Struct|BreakSCitizen _returnvalue)))) (.Name (Utilities|Struct|BreakSOfficialCitizenInfo (.OfficialInfo (Utilities|Struct|BreakSCitizen _returnvalue)))) (.FirstName (Utilities|Struct|BreakSOfficialCitizenInfo (.OfficialInfo (Utilities|Struct|BreakSCitizen _returnvalue)))) (.BirthPlace (Utilities|Struct|BreakSOfficialCitizenInfo (.OfficialInfo (Utilities|Struct|BreakSCitizen _returnvalue)))) (.Birthdate (Utilities|Struct|BreakSOfficialCitizenInfo (.OfficialInfo (Utilities|Struct|BreakSCitizen _returnvalue)))) (.Adress (Utilities|Struct|BreakSOfficialCitizenInfo (.OfficialInfo (Utilities|Struct|BreakSCitizen _returnvalue)))) (.Sexe (Utilities|Struct|BreakSOfficialCitizenInfo (.OfficialInfo (Utilities|Struct|BreakSCitizen _returnvalue)))) (.Height (Utilities|Struct|BreakSOfficialCitizenInfo (.OfficialInfo (Utilities|Struct|BreakSCitizen _returnvalue)))))))))

(fn SearchExistinData
  (params (RowData :type String%20%28by%20ref%29) (Search :type Text%20%28by%20ref%29))
  (bind _returnvalue (Utilities|String|ToString(Text) Search))
  (bind _returnvalue_2 (Utilities|String|ToLower _returnvalue))
  (return (and (Utilities|String|Contains (Utilities|String|ToLower RowData) _returnvalue_2) (not (Utilities|Array|IsEmpty _returnvalue_2)))))

(fn GetDataRowName
  (params (Table :type Data%20Table%20Object%20Reference))
  (bind _outrownames (DataTable|GetDataTableRowNames Table))
  (bind _array_element (Utilities|Array|ForEachLoopwithBreak _outrownames)
    (:LoopBody
      (bind _array (Get|GetCitizenData Table _array_element))
      (return _array _array_element))))

(fn BindAllEvent
  (CallFunction|BindReseacrchBar)
  (CallFunction|BindButtonSearch)
  (CallFunction|BindNewInvestigation))

(fn SetMaangerVariable
  (bind _scenemanager (Variables|Manager|GetSceneManager))
  (Utilities|FlowControl|Sequence
    (:then_0
      (Variables|Manager|SetData%20Manager (Variables|/Game/Blueprint/Global/Manager/BP_SceneManager.BP_SceneManager_C|GetDataManager _scenemanager))
      (Variables|Manager|SetUIManager (Variables|/Game/Blueprint/Global/Manager/BP_SceneManager.BP_SceneManager_C|GetUIManager _scenemanager))
      (Variables|Manager|SetInvestigation%20Manager (Variables|/Game/Blueprint/Global/Manager/BP_SceneManager.BP_SceneManager_C|GetInvestigation%20Manager _scenemanager)))
    (:then_1
      (Variables|Widget|SetDataCenterWidget (Variables|/Game/Widget/HUBScreen/WBP_HUBScreen.WBP_HUBScreen_C|GetWBP_DataCenter (Variables|/Game/Blueprint/Global/BP_TomorrowsDay_PC.BP_TomorrowsDay_PC_C|GetHUBScreen (Variables|Manager|GetTomorrows%20Day%20PC)))))))