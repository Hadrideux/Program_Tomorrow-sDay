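; Citizen data component that searches the citizen data table from DataManager for entries matching a search term.
; SearchData walks every row, and GetDataCitizen flattens its personal and official fields, including relations and family, into one searchable array.
; The inherited SearchExistInData tests each field; a match stops that row's field scan and passes the row name and data to CitizenDataFind, which defers to the parent.
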(event Custom|SearchData
  (params (SearchName :type Name))
  (bind _datamanager (Variables|Default|GetDataManager))
  (bind _alldatatable (Variables|/Game/Blueprint/Global/Manager/BP_DataManager.BP_DataManager_C|GetAllDataTable _datamanager))
  (bind _value (Utilities|Map|Find _alldatatable "NewEnumerator1"))
  (bind _citizenrownames (CallFunction|GetDataRowName _value))
  (bind _array_element (Utilities|Array|ForEachLoopwithBreak _citizenrownames :!label _label)
    (:LoopBody
      (bind (_array _out_row) (CallFunction|GetDataCitizen _value _array_element))
      (bind _array_element_2 (Utilities|Array|ForEachLoopwithBreak _array :!label _label_2)
        (:LoopBody
          (bind _searchcontains (CallFunction|SearchExistinData _array_element_2 (Utilities|Text|ToText(Name) SearchName)))
          (if _searchcontains
            (Utilities|FlowControl|Sequence
              (:then_0
                (goto _label Break))
              (:then_1
                (CallFunction|CitizenDataFind _array_element _out_row)))))))
    (:Completed
      (goto _label_2 Break))))

(event EventBeginPlay
  (|CallParentFunction))

(fn CitizenDataFind
  (params (CitizenName :type Name :default "None") (CitizenDataFind :type S%20Citizen%20Data%20Structure))
  (|CallParentFunction CitizenName CitizenDataFind))

(fn GetDataCitizen
  (params (DataTable :type Data%20Table%20Object%20Reference) (RowName :type Name))
  (bind _returnvalue (Utilities|GetDataTableRow DataTable RowName)
    (:then
      (Utilities|Array|AppendArray (Utilities|Array|MakeArray (.Work (Utilities|Struct|BreakSPersonalData (.PersonnalInfo (Utilities|Struct|BreakSCitizenData _returnvalue)))) (.Activity (Utilities|Struct|BreakSPersonalData (.PersonnalInfo (Utilities|Struct|BreakSCitizenData _returnvalue)))) (.Habits (Utilities|Struct|BreakSPersonalData (.PersonnalInfo (Utilities|Struct|BreakSCitizenData _returnvalue)))) (.IdentityNumber (Utilities|Struct|BreakSIdentityData (.OfficialInfo (Utilities|Struct|BreakSCitizenData _returnvalue)))) (.Name (Utilities|Struct|BreakSIdentityData (.OfficialInfo (Utilities|Struct|BreakSCitizenData _returnvalue)))) (.FirstName (Utilities|Struct|BreakSIdentityData (.OfficialInfo (Utilities|Struct|BreakSCitizenData _returnvalue)))) (.BirthPlace (Utilities|Struct|BreakSIdentityData (.OfficialInfo (Utilities|Struct|BreakSCitizenData _returnvalue)))) (.Birthdate (Utilities|Struct|BreakSIdentityData (.OfficialInfo (Utilities|Struct|BreakSCitizenData _returnvalue)))) (.Adress (Utilities|Struct|BreakSIdentityData (.OfficialInfo (Utilities|Struct|BreakSCitizenData _returnvalue)))) (.Sexe (Utilities|Struct|BreakSIdentityData (.OfficialInfo (Utilities|Struct|BreakSCitizenData _returnvalue)))) (.Height (Utilities|Struct|BreakSIdentityData (.OfficialInfo (Utilities|Struct|BreakSCitizenData _returnvalue))))) (.Relation (Utilities|Struct|BreakSPersonalData (.PersonnalInfo (Utilities|Struct|BreakSCitizenData _returnvalue)))))
      (Utilities|Array|AppendArray (Utilities|Array|MakeArray (.Work (Utilities|Struct|BreakSPersonalData (.PersonnalInfo (Utilities|Struct|BreakSCitizenData _returnvalue)))) (.Activity (Utilities|Struct|BreakSPersonalData (.PersonnalInfo (Utilities|Struct|BreakSCitizenData _returnvalue)))) (.Habits (Utilities|Struct|BreakSPersonalData (.PersonnalInfo (Utilities|Struct|BreakSCitizenData _returnvalue)))) (.IdentityNumber (Utilities|Struct|BreakSIdentityData (.OfficialInfo (Utilities|Struct|BreakSCitizenData _returnvalue)))) (.Name (Utilities|Struct|BreakSIdentityData (.OfficialInfo (Utilities|Struct|BreakSCitizenData _returnvalue)))) (.FirstName (Utilities|Struct|BreakSIdentityData (.OfficialInfo (Utilities|Struct|BreakSCitizenData _returnvalue)))) (.BirthPlace (Utilities|Struct|BreakSIdentityData (.OfficialInfo (Utilities|Struct|BreakSCitizenData _returnvalue)))) (.Birthdate (Utilities|Struct|BreakSIdentityData (.OfficialInfo (Utilities|Struct|BreakSCitizenData _returnvalue)))) (.Adress (Utilities|Struct|BreakSIdentityData (.OfficialInfo (Utilities|Struct|BreakSCitizenData _returnvalue)))) (.Sexe (Utilities|Struct|BreakSIdentityData (.OfficialInfo (Utilities|Struct|BreakSCitizenData _returnvalue)))) (.Height (Utilities|Struct|BreakSIdentityData (.OfficialInfo (Utilities|Struct|BreakSCitizenData _returnvalue))))) (.Family (Utilities|Struct|BreakSPersonalData (.PersonnalInfo (Utilities|Struct|BreakSCitizenData _returnvalue)))))
      (return (Utilities|Array|MakeArray (.Work (Utilities|Struct|BreakSPersonalData (.PersonnalInfo (Utilities|Struct|BreakSCitizenData _returnvalue)))) (.Activity (Utilities|Struct|BreakSPersonalData (.PersonnalInfo (Utilities|Struct|BreakSCitizenData _returnvalue)))) (.Habits (Utilities|Struct|BreakSPersonalData (.PersonnalInfo (Utilities|Struct|BreakSCitizenData _returnvalue)))) (.IdentityNumber (Utilities|Struct|BreakSIdentityData (.OfficialInfo (Utilities|Struct|BreakSCitizenData _returnvalue)))) (.Name (Utilities|Struct|BreakSIdentityData (.OfficialInfo (Utilities|Struct|BreakSCitizenData _returnvalue)))) (.FirstName (Utilities|Struct|BreakSIdentityData (.OfficialInfo (Utilities|Struct|BreakSCitizenData _returnvalue)))) (.BirthPlace (Utilities|Struct|BreakSIdentityData (.OfficialInfo (Utilities|Struct|BreakSCitizenData _returnvalue)))) (.Birthdate (Utilities|Struct|BreakSIdentityData (.OfficialInfo (Utilities|Struct|BreakSCitizenData _returnvalue)))) (.Adress (Utilities|Struct|BreakSIdentityData (.OfficialInfo (Utilities|Struct|BreakSCitizenData _returnvalue)))) (.Sexe (Utilities|Struct|BreakSIdentityData (.OfficialInfo (Utilities|Struct|BreakSCitizenData _returnvalue)))) (.Height (Utilities|Struct|BreakSIdentityData (.OfficialInfo (Utilities|Struct|BreakSCitizenData _returnvalue))))) _returnvalue))))

(fn SearchExistinData
  (params (RowData :type String) (Search :type Text))
  (bind _searchcontains (|CallParentFunction RowData Search))
  (return _searchcontains))