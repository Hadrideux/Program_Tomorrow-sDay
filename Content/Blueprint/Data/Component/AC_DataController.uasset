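; AC_DataController is a data component with helpers for citizen record search, DataTable row names and forwarding found data to DataManager.
; On BeginPlay it hooks SceneManager's manager-initiation event to cache InvestigationManager.
; Search is a lowercase substring match that rejects empty terms, and DataFind broadcasts results through OnSendData.
; Investigation binding is unfinished: its events are empty, and the DT_Mission start logic is disconnected.
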(event Custom|BindNewInvestigation)

(event Custom|BindInit
  (bind _output_get (Variables|Default|SetScene%20Manager (.AsBP%20Scene%20Manager (Utilities|Casting|CastToBP_SceneManager (CallFunction|GetSingletonInstance "/Game/Blueprint/Global/Manager/BP_SceneManager.BP_SceneManager_C")))))
  (EventDispatchers|AssignOnInitiateManagerEvent _output_get (delegate Custom|BindInitEvent)))

(event Custom|AddnewInvestigation)

(event Custom|BindInitEvent
  (Utilities|FlowControl|Sequence
    (:then_0
      (CallFunction|SetManagerVariable (Variables|Default|GetScene%20Manager)))))

(event EventBeginPlay
  (CallFunction|BindInit))

(fn SearchExistinCitizenData
  (params (RowData :type String) (Search :type Text))
  (bind _returnvalue (Utilities|String|ToString(Text) Search))
  (bind _returnvalue_2 (Utilities|String|ToLower _returnvalue))
  (return (and (Utilities|String|Contains (Utilities|String|ToLower RowData) _returnvalue_2) (not (Utilities|Array|IsEmpty _returnvalue_2)))))

(fn GetDataRowName
  (params (DataTable :type Data%20Table%20Object%20Reference))
  (bind _outrownames (DataTable|GetDataTableRowNames DataTable))
  (return _outrownames))

(fn DataFind
  (params (CitizenName :type Name) (CitizenDataFind :type S%20Citizen%20Data%20Structure))
  (Default|CallOnSendData (Variables|Default|GetDataManager) CitizenName CitizenDataFind))

(fn BindAllEvent
  (CallFunction|BindNewInvestigation))

(fn SetManagerVariable
  (params (SceneManager :type BP%20Scene%20Manager%20Object%20Reference))
  (Variables|Default|SetInvestigation%20Manager (Variables|/Game/Blueprint/Global/Manager/BP_SceneManager.BP_SceneManager_C|GetInvestigationManager SceneManager)))