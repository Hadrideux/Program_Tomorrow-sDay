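; Player controller for Tomorrow's Day that relays Enhanced Input and switches the player between the character and a camera controller pawn.
; On scene manager initiation it adds the input mapping contexts, then forwards look, interact and focus actions through call events.
; A FlipFlop toggles possession, camera UI, cursor, mapping contexts and input mode.
; PossessNewPawn instead blends the view, clears widgets and possesses after a matching delay.
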(event Custom|Initiate
  (CallFunction|AddDefaultMapping[Debug])
  (CallFunction|InputMappingInitiate))

(event Custom|OnChangePossesPawn_Event
  (EventDispatchers|BindEventtoOnChangePossesPawn (delegate Custom|LeaveScreen_Event)))

(event Custom|LeaveScreen_Event
  (CallFunction|PossessNewPawn (Variables|ChangePawn|GetCharacterController)))

(event Custom|SetPossessTransistion
  (params (PawnPossessed :type Pawn%20Object%20Reference))
  (Game|Player|SetViewTargetwithBlend PawnPossessed 0.5 "VTBlend_EaseOut" 1.25 false)
  (Viewport|RemoveAllWidgets))

(event Custom|PossessNewPawn
  (params (PawnPossessed :type Pawn%20Object%20Reference))
  (CallFunction|SetPossessTransistion PawnPossessed)
  (Utilities|FlowControl|Delay 0.5)
  (Pawn|Possess 0)
  (if (!= PawnPossessed self)
    (CallFunction|AddMappingContext "/Game/Blueprint/Character/Input/IMC_Default.IMC_Default")
    (CallFunction|RemoveMappingContext "/Game/Blueprint/Character/Input/IMC_Camera.IMC_Camera")
    (Input|SetInputModeGameandUI 0 (Variables|Default|GetCurrentActiveWidget) "DoNotLock" true false)
    (else
      (CallFunction|AddMappingContext "/Game/Blueprint/Character/Input/IMC_Camera.IMC_Camera")
      (CallFunction|RemoveMappingContext "/Game/Blueprint/Character/Input/IMC_Default.IMC_Default")
      (Input|SetInputModeGameOnly 0 false))))

(event Input|EnhancedActionEvents|EnhancedInputActionIA_LookAt
  (params (ActionValue :type Vector%202D%20Structure) (ElapsedSeconds :type Float%20%28double-precision%29) (TriggeredSeconds :type Float%20%28double-precision%29) (InputAction :type Input%20Action%20Object%20Reference :default "/Game/Blueprint/Character/Input/Action/Game/Player/IA_LookAt.IA_LookAt"))
  ;[0.04911 0.6101 1] LookAt
  (Default|CallOnLookat ActionValue))

(event Input|EnhancedActionEvents|EnhancedInputActionIA_Interact
  (params (ActionValue :type Boolean) (ElapsedSeconds :type Float%20%28double-precision%29) (TriggeredSeconds :type Float%20%28double-precision%29) (InputAction :type Input%20Action%20Object%20Reference :default "/Game/Blueprint/Character/Input/Action/Game/Player/IA_Interact.IA_Interact"))
  (:Started
    (Default|CallOnPlayerInteract)))

(event Input|EnhancedActionEvents|EnhancedInputActionIA_Focus
  (params (ActionValue :type Boolean) (ElapsedSeconds :type Float%20%28double-precision%29) (TriggeredSeconds :type Float%20%28double-precision%29) (InputAction :type Input%20Action%20Object%20Reference :default "/Game/Blueprint/Character/Input/Action/Game/Camera/IA_Focus.IA_Focus"))
  (:Started
    (Default|CallOnFocusCameraElement)))

(event Input|EnhancedActionEvents|EnhancedInputActionIA_ChangePawn
  (params (ActionValue :type Boolean) (ElapsedSeconds :type Float%20%28double-precision%29) (TriggeredSeconds :type Float%20%28double-precision%29) (InputAction :type Input%20Action%20Object%20Reference :default "/Game/Blueprint/Character/Input/Action/Debug/IA_ChangePawn.IA_ChangePawn"))
  (bind _self self)
  (bind _scene_manager (Variables|Manager|GetScene%20Manager))
  (bind _cameraactormanager (Variables|/Game/Blueprint/Global/Manager/BP_SceneManager.BP_SceneManager_C|GetCameraActorManager _scene_manager))
  (:Started
    (Utilities|FlowControl|FlipFlop
      (:A
        (Pawn|Possess (Variables|ChangePawn|GetCameraController))
        (Default|DisplayCameraInterface _cameraactormanager)
        (Variables|Default|SetbShowMouseCursor true)
        (CallFunction|AddMappingContext "/Game/Blueprint/Character/Input/IMC_Camera.IMC_Camera")
        (CallFunction|RemoveMappingContext "/Game/Blueprint/Character/Input/IMC_Default.IMC_Default")
        (Input|SetInputModeGameandUI _self (Variables|/Game/Blueprint/Global/Manager/BP_CameraActorManager.BP_CameraActorManager_C|GetCameraInterface _cameraactormanager) "DoNotLock" true false))
      (:B
        (Pawn|Possess (Variables|ChangePawn|GetCharacterController))
        (Default|RemoveCameraInterface _cameraactormanager)
        (Variables|Default|SetbShowMouseCursor false)
        (CallFunction|AddMappingContext "/Game/Blueprint/Character/Input/IMC_Default.IMC_Default")
        (CallFunction|RemoveMappingContext "/Game/Blueprint/Character/Input/IMC_Camera.IMC_Camera")
        (Input|SetInputModeGameOnly _self false)))))

(event EventBeginPlay
  (bind _output_get (Variables|Manager|SetScene%20Manager (CallFunction|InitiateSceneManager)))
  (EventDispatchers|BindEventtoOnInitiateManagerEvent _output_get (delegate Custom|Initiate)))

(fn ConstructionScript)

(fn InputMappingInitiate
  (for _array_element (Variables|Mapping|GetMapping%20Context)
    (Input|AddMappingContext (PlayerController|LocalPlayerSubsystems|GetEnhancedInputLocalPlayerSubsystem) _array_element 0 "(bIgnoreAllPressedKeysUntilRelease=True,bForceImmediately=False,bNotifyUserSettings=False)")))

(fn AddMappingContext
  (params (MappingContext :type Input%20Mapping%20Context%20Object%20Reference))
  (Input|AddMappingContext (PlayerController|LocalPlayerSubsystems|GetEnhancedInputLocalPlayerSubsystem) MappingContext 0 "(bIgnoreAllPressedKeysUntilRelease=True,bForceImmediately=False,bNotifyUserSettings=False)"))

(fn RemoveMappingContext
  (params (MappingContext :type Input%20Mapping%20Context%20Object%20Reference))
  (Input|RemoveMappingContext (PlayerController|LocalPlayerSubsystems|GetEnhancedInputLocalPlayerSubsystem) MappingContext "(bIgnoreAllPressedKeysUntilRelease=True,bForceImmediately=False,bNotifyUserSettings=False)"))

(fn AddDefaultMapping[Debug]
  (Input|AddMappingContext (PlayerController|LocalPlayerSubsystems|GetEnhancedInputLocalPlayerSubsystem) "/Game/Blueprint/Character/Input/IMC_Default.IMC_Default" 0 "(bIgnoreAllPressedKeysUntilRelease=True,bForceImmediately=False,bNotifyUserSettings=False)"))