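; BP_TomorrwsDay_PC is a player controller that sets up Enhanced Input and relays player input as events.
; On BeginPlay it creates and stores a scene manager, then adds the default mapping context once that manager signals initiation.
; Look-at and interact input actions are rebroadcast through OnLookAt and OnPlayerInteract calls for other objects to handle.
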(event Custom|Initiate
  (CallFunction|InputMappingInitiate))

(event Input|EnhancedActionEvents|EnhancedInputActionIA_LookAt
  (params (ActionValue :type Vector%202D%20Structure) (ElapsedSeconds :type Float%20%28double-precision%29) (TriggeredSeconds :type Float%20%28double-precision%29) (InputAction :type Input%20Action%20Object%20Reference :default "/Game/Blueprint/Character/Input/Action/Game/IA_LookAt.IA_LookAt"))
  ;[1 1 1] LookAt
  (Default|CallOnLookat ActionValue))

(event Input|EnhancedActionEvents|EnhancedInputActionIA_Interact
  (params (ActionValue :type Boolean) (ElapsedSeconds :type Float%20%28double-precision%29) (TriggeredSeconds :type Float%20%28double-precision%29) (InputAction :type Input%20Action%20Object%20Reference :default "/Game/Blueprint/Character/Input/Action/Game/IA_Interact.IA_Interact"))
  (Default|CallOnPlayerInteract))

(event EventBeginPlay
  (bind _scene_manager (CallFunction|InitiateSceneManager))
  (Utilities|FlowControl|Sequence
    (:then_0
      (Variables|Default|SetScene%20Manager _scene_manager))
    (:then_1
      (EventDispatchers|BindEventtoOnInitiateManagerEvent _scene_manager (delegate Custom|Initiate)))))

(fn ConstructionScript)

(fn InputMappingInitiate
  (Input|AddMappingContext (PlayerController|LocalPlayerSubsystems|GetEnhancedInputLocalPlayerSubsystem) "/Game/Blueprint/Character/Input/IMC_Default.IMC_Default" 0 "(bIgnoreAllPressedKeysUntilRelease=True,bForceImmediately=False,bNotifyUserSettings=False)"))