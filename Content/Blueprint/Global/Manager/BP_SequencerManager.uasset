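; Sequencer manager that creates a level sequence player and controls its playback from sequencer state changes.
; Once the scene manager initializes, it caches the game state manager, binds the sequence-state event and creates the player.
; States play, pause or change play rate; REVERSED only slows playback, as PlayReverse is unwired.
; A game-state handler toggles a playable flag, but its binding event is never called here.
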(event Custom|Initialization_Event
  (Utilities|FlowControl|Sequence
    (:then_0
      (Init|SetManagerVariable))
    (:then_1
      (Init|BindAllEvent))
    (:then_2
      (bind _returnvalue (Sequencer|Player|CreateLevelSequencePlayer (Variables|Sequence|GetLevelSequence)))
      (Variables|Sequence|SetCurrent%20Level%20Sequence _returnvalue))))

(event Custom|BindSequenceState
  (EventDispatchers|BindEventtoOnSequenceStateChange (delegate Custom|SequenceStateChange_Event)))

(event Custom|SequenceStateChange_Event
  (params (SequencerState :type ESequencerState%20Enum :default "NewEnumerator0"))
  (bind _current_level_sequence (Variables|Sequence|GetCurrent%20Level%20Sequence))
  (switch Utilities|FlowControl|Switch|SwitchonESequencerState SequencerState
    (:NewEnumerator1
      (Sequencer|Player|Play _current_level_sequence :!class /Script/MovieScene.MovieSceneSequencePlayer))
    (:NewEnumerator2
      (Sequencer|Player|Pause _current_level_sequence))
    (:NewEnumerator3
      (Components|Timeline|SetPlayRate _current_level_sequence 0.2))
    (:NewEnumerator4
      (Components|Timeline|SetPlayRate _current_level_sequence 2.0))))

(event Custom|CustomEvent)

(event Custom|BindGameState
  (EventDispatchers|AssignOnGameStateChange (Variables|Manager|GetGame%20State%20Manager) (delegate Custom|GameState_Event)))

(event Custom|GameState_Event
  (params (EGameState :type EGameState%20Enum :default "NewEnumerator0"))
  (switch Utilities|FlowControl|Switch|SwitchonEGameState EGameState
    (:NewEnumerator2
      (Variables|Sequence|SetbIsSequencePlaybable false))
    (:NewEnumerator3
      (Variables|Sequence|SetbIsSequencePlaybable true :!label _label))
    (:NewEnumerator4
      (goto _label))))

(event EventBeginPlay
  (bind _output_get (Variables|Manager|SetScene%20Manager (CallFunction|InitiateSceneManager)))
  (EventDispatchers|AssignOnInitiateManagerEvent _output_get (delegate Custom|Initialization_Event)))

(fn ConstructionScript)

(fn BindAllEvent
  (CallFunction|BindSequenceState))

(fn SetManagerVariable
  (Variables|Manager|SetGame%20State%20Manager (Variables|/Game/Blueprint/Global/Manager/BP_SceneManager.BP_SceneManager_C|GetGameStateManager (Variables|Manager|GetScene%20Manager))))