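; BP_CameraActorManager is a manager that tracks the selected camera filter and shows or removes the camera interface widget.
; On BeginPlay it gets the BP_SceneManager singleton and hooks into its manager-initiation event, deferring its own event binding until that fires.
; It then listens for filter changes, storing the current filter and post-process index without applying them here.
; Separate functions add the camera interface to the viewport and remove it.
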(event Custom|BindCameraFilter
  (EventDispatchers|BindEventtoOnChangeFilter (delegate Custom|ChangeFilter_Event)))

(event Custom|ChangeFilter_Event
  (params (ESelectedFilter :type ECameraFilter%20Enum :default "NewEnumerator0") (PostProcessIndex :type Integer))
  (Variables|State|SetECurrentCameraFilter ESelectedFilter)
  (Variables|Default|SetCurrent%20PostProcess%20Index PostProcessIndex))

(event Custom|BindInit
  ;[1 1 1] Initialization
  (bind _output_get (Variables|Manager|SetScene%20Manager (.AsBP%20Scene%20Manager (Utilities|Casting|CastToBP_SceneManager (CallFunction|GetSingletonInstance "/Game/Blueprint/Global/Manager/BP_SceneManager.BP_SceneManager_C")))))
  (EventDispatchers|BindEventtoOnInitiateManagerEvent _output_get (delegate Custom|Initiate_Event)))

(event Custom|Initiate_Event
  ;[1 1 1] Initialization
  (Utilities|FlowControl|Sequence
    (:then_1
      (CallFunction|BindEvent))))

(event EventBeginPlay
  ;[1 1 1] Initialization
  (CallFunction|BindInit))

(fn ConstructionScript)

(fn DisplayCameraInterface
  (UserInterface|Viewport|AddtoViewport (Variables|Camera|GetCameraInterface) 0))

(fn RemoveCameraInterface
  (Widget|RemovefromParent (Variables|Camera|GetCameraInterface)))

(fn BindEvent
  (CallFunction|BindCameraFilter))