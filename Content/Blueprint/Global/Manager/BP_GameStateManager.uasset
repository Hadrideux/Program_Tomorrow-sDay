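; BP_GameStateManager is a manager Blueprint that passes game pause and start changes on to the sequencer manager.
; On BeginPlay it creates the scene manager and waits for its initiate event, then caches the SequencerManager reference from it.
; Its game state handler maps each state to a sequence state change call.
; BindAllEvent is empty, and nothing in this file calls BindGameStateChange, which binds that handler.
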(event Custom|Initialization_Event
  (Utilities|FlowControl|Sequence
    (:then_0
      (CallFunction|SetManagerVariable))
    (:then_1
      (CallFunction|BindAllEvent))))

(event Custom|BindGameStateChange
  (EventDispatchers|BindEventtoOnGameStateChange (delegate Custom|OnGameStateChange_Event)))

(event Custom|OnGameStateChange_Event
  (params (EGameState :type EGameState%20Enum :default "NewEnumerator0"))
  (bind _sequencer_manager (Variables|Default|GetSequencer%20Manager))
  (switch Utilities|FlowControl|Switch|SwitchonEGameState EGameState
    (:NewEnumerator1
      (Default|CallOnSequenceStateChange _sequencer_manager "NewEnumerator2"))
    (:NewEnumerator3
      (Default|CallOnSequenceStateChange _sequencer_manager "NewEnumerator1"))))

(event EventBeginPlay
  (bind _output_get (Variables|SceneManager|SetScene%20Manager (CallFunction|InitiateSceneManager)))
  (EventDispatchers|AssignOnInitiateManagerEvent _output_get (delegate Custom|Initialization_Event)))

(fn ConstructionScript)

(fn BindAllEvent)

(fn SetManagerVariable
  (Variables|Default|SetSequencer%20Manager (Variables|/Game/Blueprint/Global/Manager/BP_SceneManager.BP_SceneManager_C|GetSequencerManager (Variables|SceneManager|GetScene%20Manager))))