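; Camera component that switches the camera manager's post-process volume between no filter and Audio, Thermal or UV filters.
; SetSelectedFilter zeroes the tracked CurrentFilter material's blend weight, then sets the material at the given index to full weight and tracks it.
; Each weight change rebuilds the post-process settings from the materials array.
; Every selection then reapplies manual metering and a fixed exposure compensation.
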(fn GetPostProcessVolume
  (params (CameraManager :type BP%20Camera%20Manager%20Object%20Reference))
  (return (Variables|/Script/Engine.PostProcessVolume|GetSettings (Variables|/Game/Blueprint/Global/Manager/BP_CameraManager.BP_CameraManager_C|GetPostProcessVolume CameraManager))))

(fn SetSelectedFilter
  (params (GetFilterType :type EFilterType%20Enum :default "NewEnumerator0") (PostProcessIndex :type Integer) (CameraManager :type BP%20Camera%20Manager%20Object%20Reference))
  (switch Utilities|FlowControl|Switch|SwitchonEFilterType GetFilterType
    (:NewEnumerator0
      (bind _setsettings (PostProcess|DeactivePreviousFilter (PostProcess|GetPostProcessVolume CameraManager)))
      (bind _output_get (Variables|/Script/Engine.PostProcessVolume|SetSettings (Variables|/Game/Blueprint/Global/Manager/BP_CameraManager.BP_CameraManager_C|GetPostProcessVolume CameraManager) _setsettings)))
    (:NewEnumerator1
      (PostProcess|EnablePostProcess PostProcessIndex CameraManager))
    (:NewEnumerator2
      (PostProcess|EnablePostProcess PostProcessIndex CameraManager))
    (:NewEnumerator3
      (PostProcess|EnablePostProcess PostProcessIndex CameraManager)))
  (|SetBy-RefVar (.AutoExposureMethod (Utilities|Struct|BreakPostProcessSettings _output_get)) "AEM_Manual")
  (|SetBy-RefVar (.AutoExposureBias (Utilities|Struct|BreakPostProcessSettings _output_get)) 9.5))

(fn EnablePostProcess
  (params (PostProcessIndex :type Integer) (CameraManager :type BP%20Camera%20Manager%20Object%20Reference))
  (bind _settings (PostProcess|GetPostProcessVolume CameraManager))
  (bind _postprocessvolume (Variables|/Game/Blueprint/Global/Manager/BP_CameraManager.BP_CameraManager_C|GetPostProcessVolume CameraManager))
  (bind _setsettings (PostProcess|DeactivePreviousFilter _settings))
  (Variables|/Script/Engine.PostProcessVolume|SetSettings _postprocessvolume _setsettings)
  (bind _setsettings_2 (PostProcess|ActiveNewFilter _settings PostProcessIndex))
  (Variables|/Script/Engine.PostProcessVolume|SetSettings _postprocessvolume _setsettings_2))

(fn DeactivePreviousFilter
  (params (GetSettings :type Post%20Process%20Settings%20Structure))
  (bind _weightedblendables (Utilities|Struct|BreakPostProcessSettings GetSettings))
  (bind _currentfilter (Variables|Default|GetCurrentFilter))
  (bind _array (Utilities|Struct|BreakWeightedBlendables _weightedblendables))
  (bind _returnvalue (Utilities|Array|FindItem _array _currentfilter))
  (if (!= _returnvalue 0)
    (bind _postprocesssettings (PostProcess|SetPostProcessFilter _array _returnvalue 0.0))
    (return _postprocesssettings)))

(fn ActiveNewFilter
  (params (GetSettings :type Post%20Process%20Settings%20Structure%20%28by%20ref%29) (WeightIndex :type Integer))
  (bind _weightedblendables (Utilities|Struct|BreakPostProcessSettings GetSettings))
  (bind _array (Utilities|Struct|BreakWeightedBlendables _weightedblendables))
  (bind _postprocesssettings (PostProcess|SetPostProcessFilter _array WeightIndex 1.0))
  (Variables|Default|SetCurrentFilter (Utilities|Array|Get(acopy) _array WeightIndex))
  (return _postprocesssettings))

(fn SetPostProcessFilter
  (params (PostProcess :type Array%20of%20Weighted%20Blendable%20Structures) (PostProcessIndex :type Integer) (PostProcessWeight :type Float%20%28single-precision%29))
  (Utilities|Array|SetArrayElem PostProcess PostProcessIndex (Utilities|Struct|MakeWeightedBlendable PostProcessWeight (.object (Utilities|Array|Get(acopy) PostProcess PostProcessIndex))))
  (return (Utilities|Struct|MakePostProcessSettings (Utilities|Struct|MakeWeightedBlendables PostProcess))))

(fn SetPostProcessVolume
  (params (CameraManager :type BP%20Camera%20Manager%20Object%20Reference) (Item :type Weighted%20Blendable%20Structure%20%28by%20ref%29) (Index :type Integer))
  (Utilities|Array|SetArrayElem (Utilities|Struct|BreakWeightedBlendables (Utilities|Struct|BreakPostProcessSettings (Variables|/Script/Engine.PostProcessVolume|GetSettings (Variables|/Game/Blueprint/Global/Manager/BP_CameraManager.BP_CameraManager_C|GetPostProcessVolume CameraManager)))) Index Item))