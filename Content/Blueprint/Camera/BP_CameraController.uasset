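; Surveillance-style camera controller actor that moves between preset camera positions, carries a render-target scene capture, and analyses hints.
; Once the scene manager initializes, it caches managers, registers with the player controller, and binds camera manager events.
; Selected hints route by type to UV, thermal or audio filter components, with citizen hints sharing audio.
; Focus only prints the mouse-traced actor's name, and the filter-change binding is never called.
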(event Custom|BindFocusElement
  (EventDispatchers|BindEventtoOnFocusCameraElement (Variables|Manager|GetTomorrows%20Day%20PC) (delegate Custom|FocusCamera_Event)))

(event Custom|FocusCamera_Event
  (bind _hitactor (SelectionHint|MousePositiontoWorldLocation))
  (Development|PrintString (Utilities|GetDisplayName _hitactor)))

(event Custom|Initialization_Event
  ;[1 1 1] Initialization Binding Event
  (Utilities|FlowControl|Sequence
    (:then_0
      (Initiate|SetManagerVariable)
      (Variables|/Game/Blueprint/Global/BP_TomorrowsDay_PC.BP_TomorrowsDay_PC_C|SetCameraController (Variables|Manager|GetTomorrows%20Day%20PC) self))
    (:then_1
      (Initiate|BindAllEvent))
    (:then_2
      (CameraOption|SwitchCameraLocation))))

(event EventBeginPlay
  ;[1 1 1] Initialization Binding Event
  (bind _output_get (Variables|Manager|SetScene%20Manager (CallFunction|InitiateSceneManager)))
  (EventDispatchers|BindEventtoOnInitiateManagerEvent _output_get (delegate Custom|Initialization_Event)))

(event Custom|OnAnalyseSelect_Event
  (params (HintSelect :type BP%20A%20Hint%20Controller%20Object%20Reference))
  ;[1 1 1] Set Analyse
  (CameraOption|SwitchFilterMode HintSelect))

(event Custom|BindAnalyse
  ;[1 1 1] Set Analyse
  (EventDispatchers|AssignOnAnalyseSelect (Variables|Manager|GetCameraActor%20Manager) (delegate Custom|OnAnalyseSelect_Event)))

(event Custom|BindChangeCamera
  ;[1 0.1098 0.0902] Change Camera Position
  (EventDispatchers|BindEventtoOnChangeCameraPositon (Variables|Manager|GetCameraActor%20Manager) (delegate Custom|ChangeCameraPosition)))

(event Custom|ChangeCameraPosition
  (params (CameraPositionIndex :type Integer))
  ;[1 0.1098 0.0902] Change Camera Position
  (CameraOption|SwitchCameraLocation CameraPositionIndex))

(event Custom|OnChangeFilter_Event
  (params (ESelectedFilter :type ECameraFilter%20Enum :default "NewEnumerator0") (PostProcessIndex :type Integer))
  ;[0.102 0.2196 1] Filter Change Event
  (Default|SetFilterVisual (Variables|Default|GetAC_CameraFilter) ESelectedFilter PostProcessIndex))

(event Custom|BindFilterEvent
  ;[0.102 0.2196 1] Filter Change Event
  (EventDispatchers|AssignOnChangeFilter (Variables|Manager|GetCameraActor%20Manager) (delegate Custom|OnChangeFilter_Event)))

(fn ConstructionScript
  (bind _scenecapturecomponent2d (Variables|Default|GetSceneCaptureComponent2D))
  (Utilities|IsValid (Variables|/Script/Engine.SceneCaptureComponent2D|GetTextureTarget _scenecapturecomponent2d)
    (:Is%20Valid
      (Variables|/Script/Engine.SceneCaptureComponent2D|SetTextureTarget _scenecapturecomponent2d "/Game/Asset/Texture/CameraView/RT_CameraView.RT_CameraView"))))

(fn SwitchCameraLocation
  (params (Position :type Integer))
  (bind _cameraactor_manager (Variables|Manager|GetCameraActor%20Manager))
  (bind _cameraposition (Variables|/Game/Blueprint/Global/Manager/BP_CameraActorManager.BP_CameraActorManager_C|GetCameraPosition _cameraactor_manager))
  (bind _output (Utilities|Array|Get(acopy) _cameraposition Position))
  (Utilities|IsValid _output
    (:Is%20Valid
      (Transformation|SetActorTransform self (Transformation|GetActorTransform _output) true))))

(fn MousePositiontoWorldLocation
  (bind _returnvalue (Game|GetPlayerController 0))
  (bind (_worldlocation _worlddirection) (Game|Player|ConvertMouseLocationToWorldSpace _returnvalue))
  (bind _outhit (Collision|SphereTraceByChannel _worldlocation (+ _worldlocation (* _worlddirection 2e+03)) (Variables|DebugLineTrace|GetRadius%20Spehre%20Trace) (Variables|DebugLineTrace|GetTrace%20Channel) false 0 (Variables|DebugLineTrace|GetDraw%20Debug%20Type)))
  (return (.HitActor (Collision|BreakHitResult _outhit))))

(fn BindAllEvent
  (Utilities|FlowControl|Sequence
    (:then_0
      (CallFunction|BindChangeCamera)
      (CallFunction|BindChangeCamera))
    (:then_1
      (CallFunction|BindAnalyse)
      (CallFunction|BindFocusElement))))

(fn SetManagerVariable
  (bind _scene_manager (Variables|Manager|GetScene%20Manager))
  (Utilities|FlowControl|Sequence
    (:then_0
      (Variables|Manager|SetTomorrows%20Day%20PC (.AsBP%20Tomorrows%20Day%20PC (Utilities|Casting|CastToBP_TomorrowsDay_PC (Game|GetPlayerController 0)))))
    (:then_1
      (Variables|Manager|SetUIManager (Variables|/Game/Blueprint/Global/Manager/BP_SceneManager.BP_SceneManager_C|GetUIManager _scene_manager))
      (Variables|Manager|SetCameraActor%20Manager (Variables|/Game/Blueprint/Global/Manager/BP_SceneManager.BP_SceneManager_C|GetCameraActorManager _scene_manager))
      (Variables|Manager|SetSequencer%20Manager (Variables|/Game/Blueprint/Global/Manager/BP_SceneManager.BP_SceneManager_C|GetSequencerManager _scene_manager)))))

(fn SequenceControl
  (params (SequencerState :type ESequencerState%20Enum :default "NewEnumerator0"))
  (Default|CallOnSequenceStateChange (Variables|Manager|GetSequencer%20Manager) SequencerState))

(fn SwitchFilterMode
  (params (Selected%20Hint :type BP%20A%20Hint%20Controller%20Object%20Reference))
  (switch Utilities|FlowControl|Switch|SwitchonEHintType (Variables|/Game/Blueprint/Hint/BP_AHintController.BP_AHintController_C|GetEHintType Selected%20Hint)
    (:NewEnumerator1
      (bind _asbp_uvhint_controller (Utilities|Casting|CastToBP_UVHintController Selected%20Hint))
      (Default|AnalyseUVSource (Variables|Default|GetAC_UVFilter) _asbp_uvhint_controller))
    (:NewEnumerator2
      (bind _asbp_thermal_hint_controller (Utilities|Casting|CastToBP_ThermalHintController Selected%20Hint))
      (Default|AnalyseThermalSource (Variables|Default|GetAC_ThermalFilter) _asbp_thermal_hint_controller))
    (:NewEnumerator3
      (bind _asbp_audio_hint_controller (Utilities|Casting|CastToBP_AudioHintController Selected%20Hint :!label _label))
      (Default|AnalyseAudioSource (Variables|Default|GetAC_AudioFilter) "NewEnumerator2" _asbp_audio_hint_controller))
    (:NewEnumerator4
      (goto _label))))