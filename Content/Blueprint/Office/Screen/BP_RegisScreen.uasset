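; BP_RegisScreen is an office screen Blueprint that shows the WBP_RegisInterface widget and reacts to analyse selection from the camera manager.
; On BeginPlay it binds to the singleton BP_SceneManager's initiate event, which then caches the CameraActorManager and binds to its OnAnalyseSelect dispatcher.
; When that fires, it switches the widget's InterfaceSwitcher to its second page, ignoring the hint argument.
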(event Custom|BindCameraSelected
  ;[0.6146 0 0.02394] ??????
  (EventDispatchers|AssignOnAnalyseSelect (Variables|Manager|GetCamera%20Manager) (delegate Custom|OnAnalyseSelect_Event)))

(event Custom|CameraSelected_Event
  (params (bIsSelected :type Boolean))
  ;[0.6146 0 0.02394] ??????
)

(event Custom|OnInitiateManagerEvent_Event
  ;[0.04911 0.6101 1] Initialization Binding Event
  (Utilities|FlowControl|Sequence
    (:then_0
      (CallFunction|SetManagerVariable))
    (:then_1
      (CallFunction|BindAllEvent))))

(event Custom|OnAnalyseSelect_Event
  (params (HintSelect :type BP%20A%20Hint%20Controller%20Object%20Reference))
  ;[0.6146 0 0.02394] ??????
  (bind _aswbp_regis_interface (Utilities|Casting|CastToWBP_RegisInterface (UserInterface|GetWidget (Variables|Default|GetWidget))))
  (Class|WidgetSwitcher|SetActiveWidgetIndex (Variables|/Game/Widget/RegisScreen/WBP_RegisInterface.WBP_RegisInterface_C|GetInterfaceSwitcher _aswbp_regis_interface) 1))

(event Custom|BindInit
  ;[0.04911 0.6101 1] Initialization Binding Event
  (bind _output_get (Variables|Manager|SetScene%20Manager (.AsBP%20Scene%20Manager (Utilities|Casting|CastToBP_SceneManager (CallFunction|GetSingletonInstance "/Game/Blueprint/Global/Manager/BP_SceneManager.BP_SceneManager_C")))))
  (EventDispatchers|AssignOnInitiateManagerEvent _output_get (delegate Custom|OnInitiateManagerEvent_Event)))

(event EventBeginPlay
  ;[0.04911 0.6101 1] Initialization Binding Event
  (CallFunction|BindInit))

(fn ConstructionScript)

(fn SetManagerVariable
  (Variables|Manager|SetCamera%20Manager (Variables|/Game/Blueprint/Global/Manager/BP_SceneManager.BP_SceneManager_C|GetCameraActorManager (Variables|Manager|GetScene%20Manager))))

(fn BindAllEvent
  (CallFunction|BindCameraSelected))