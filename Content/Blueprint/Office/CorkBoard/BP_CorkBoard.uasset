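; Office cork board actor that reveals investigation hint sheets on its HUD widget as analyses are printed.
; On BeginPlay it waits for the SceneManager singleton's initialization event, then caches the InvestigationManager and binds its analysis events.
; Each print makes the next SheetHintList entry visible by key order.
; Analysis completion clears the CurrentHint through TomorrowsDayPC, although that reference is set to None here.
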(event Custom|OnPrintAnalyse_Event
  (bind _widget (Variables|Default|GetWidget))
  (bind _returnvalue (UserInterface|GetWidget _widget))
  (bind _aswbp_cork_board_hud (Utilities|Casting|CastToWBP_CorkBoardHUD _returnvalue))
  (bind _sheethintlist (Variables|/Game/Widget/CorkBoard/WBP_CorkBoardHUD.WBP_CorkBoardHUD_C|GetSheetHintList _aswbp_cork_board_hud))
  (bind _keys (Utilities|Map|Keys _sheethintlist))
  (if (== (Variables|Default|GethintIndex) 0)
    (Widget|SetVisibility (.Value (Utilities|Map|Find _sheethintlist (Utilities|Array|Get(acopy) _keys (Variables|Default|GethintIndex)))) "Visible")
    (else
      (Widget|SetVisibility (.Value (Utilities|Map|Find _sheethintlist (Utilities|Array|Get(acopy) _keys (Variables|Default|GethintIndex)))) "Visible")))
  (Math|Integer|IncrementInt (Variables|Default|GethintIndex)))

(event Custom|OnAnalyseComplete_Event
  (params (CurrentHint :type Object%20Object%20Reference) (Analyse%20Index :type Integer))
  (Variables|/Game/Widget/CorkBoard/WBP_CorkBoardHUD.WBP_CorkBoardHUD_C|SetCurrent%20Hint (Variables|/Game/Blueprint/Global/BP_TomorrowsDay_PC.BP_TomorrowsDay_PC_C|GetCorkBoard (.Tomorrows%20Day%20PC (Variables|Default|GetTomorrows%20Day%20PC))) 0 CurrentHint))

(event Custom|BindInit
  ;[1 1 1] Initialization Binding Event
  (bind _output_get (Variables|Default|SetScene%20Manager (.AsBP%20Scene%20Manager (Utilities|Casting|CastToBP_SceneManager (.Output_Get (CallFunction|GetSingletonInstance 0 "/Game/Blueprint/Global/Manager/BP_SceneManager.BP_SceneManager_C"))))))
  (EventDispatchers|BindEventtoOnInitializationBind _output_get (delegate Custom|Init%20Event)))

(event Custom|Init%20Event
  ;[1 1 1] Initialization Binding Event
  (Utilities|FlowControl|Sequence
    (:then_0
      (CallFunction|SetManagerVariable))
    (:then_1
      (CallFunction|BindAllEvent))))

(event Custom|BindPrintAnalyse
  (EventDispatchers|AssignOnPrintAnalyse (Variables|Default|GetInvestigation%20Manager) (delegate Custom|OnPrintAnalyse_Event)))

(event Custom|BindAnalyseComplete
  (EventDispatchers|AssignOnAnalyseComplete (Variables|Default|GetInvestigation%20Manager) (delegate Custom|OnAnalyseComplete_Event)))

(event EventBeginPlay
  ;[1 1 1] Initialization Binding Event
  (CallFunction|BindInit))

(fn ConstructionScript)

(fn SetManagerVariable
  (Utilities|FlowControl|Sequence
    (:then_0
      (Variables|Default|SetInvestigation%20Manager (Variables|/Game/Blueprint/Global/Manager/BP_SceneManager.BP_SceneManager_C|GetInvestigation%20Manager (Variables|Default|GetScene%20Manager))))
    (:then_1
      (Variables|Default|SetTomorrows%20Day%20PC 0 (.AsBP%20Tomorrws%20Day%20PC (Utilities|Casting|CastToBP_TomorrowsDay_PC (Game|GetPlayerController 0)))))))

(fn BindAllEvent
  (CallFunction|BindAnalyseComplete)
  (CallFunction|BindPrintAnalyse))