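; Office radio Blueprint that can be toggled on and off to play a radio station sound.
; A toggle event checks the on/off flag and calls the matching turn-on or turn-off event, each playing a one-shot sound at the radio model's location.
; Turning on waits briefly before starting the station audio and setting the flag, while turning off stops it immediately.
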(event Custom|Turn%20Radio%20Off
  (Audio|PlaySoundatLocation 0 (Transformation|GetWorldLocation (Variables|Default|GetRadio_Model)) "0, 0, 0" 1.0 1.0 0.0 0 0 0 0)
  (Audio|Components|Audio|Stop (Variables|Default|GetSC_RadioStation))
  (Variables|Default|SetisRadioOn false))

(event Custom|Turn%20Radio%20On
  (Audio|PlaySoundatLocation 0 (Transformation|GetWorldLocation (Variables|Default|GetRadio_Model)) "0, 0, 0" 1.0 1.0 0.0 0 0 0 0)
  (Utilities|FlowControl|Delay 0.5)
  (Audio|Components|Audio|Play (Variables|Default|GetSC_RadioStation) 0.0)
  (Variables|Default|SetisRadioOn true))

(event Custom|Toggle%20Radio%20ON/OFF
  (if (Variables|Default|GetisRadioOn)
    (CallFunction|TurnRadioOff)
    (else
      (CallFunction|TurnRadioon))))

(fn ConstructionScript)