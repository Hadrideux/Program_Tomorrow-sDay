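; Controller Blueprint that plays, pauses and scrubs the current level sequence held by the SequencerManager.
; Once the SceneManager signals initialization, it caches the SequencerManager and calls two bind events, which are empty.
; Handlers switch play/pause by enum and map a normalized time to a frame between zero and the sequence end.
; The nodes binding these handlers to manager events are unconnected, so neither is bound here.
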(event Custom|BindSequencerTime
  ;[0.2672 1 0.1234] TimeCode Sequence
)

(event Custom|OnChangeTimeCcode
  (params (SequencerTime :type Float%20%28double-precision%29))
  (bind _sequencermanager (Variables|Manager|GetSequencerManager))
  (bind _currentlevelsequence (Variables|/Game/Blueprint/Global/Manager/BP_SequencerManager.BP_SequencerManager_C|GetCurrentLevelSequence _sequencermanager))
  ;[0.2672 1 0.1234] TimeCode Sequence
  (bind _output_get (Variables|Default|SetPlayBackTime (Math|Float|Lerp 0.0 (Math|Conversions|ToFloat(Integer) (.value (.frame (Class|MovieSceneSequencePlayer|GetEndTime _currentlevelsequence)))) SequencerTime)))
  (Components|Timeline|SetPlaybackPosition _currentlevelsequence (Utilities|Struct|MakeMovieSceneSequencePlaybackParams (Utilities|Struct|MakeFrameTime (Utilities|Struct|MakeFrameNumber (Math|Float|Truncate _output_get)) 0.0) _output_get "" "Frame" "Play" false)))

(event Custom|Initialization_Event
  ;[1 1 1] Initialization Binding Event
  (Utilities|FlowControl|Sequence
    (:then_0
      (CallFunction|SetManagerVariable))
    (:then_1
      (CallFunction|BindAllEvent))))

(event Custom|OnPlaySequence
  (params (Play/Pause :type Byte :default 0))
  (bind _sequencermanager (Variables|Manager|GetSequencerManager))
  (bind _currentlevelsequence (Variables|/Game/Blueprint/Global/Manager/BP_SequencerManager.BP_SequencerManager_C|GetCurrentLevelSequence _sequencermanager))
  ;[1 0.1311 0.07812] Play/Pause Sequence
  (switch Utilities|FlowControl|Switch|Switchon Play/Pause
    (:NewEnumerator1
      (Sequencer|Player|Play _currentlevelsequence :!class /Script/MovieScene.MovieSceneSequencePlayer))
    (:NewEnumerator2
      (Sequencer|Player|Pause _currentlevelsequence))))

(event Custom|BindPlaySequence
  ;[1 0.1311 0.07812] Play/Pause Sequence
)

(event EventBeginPlay
  ;[1 1 1] Initialization Binding Event
  (bind _output_get (Variables|Manager|SetScene%20Manager (CallFunction|InitiateSceneManager)))
  (EventDispatchers|BindEventtoOnInitiateManagerEvent _output_get (delegate Custom|Initialization_Event)))

(fn ConstructionScript)

(fn BindAllEvent
  (CallFunction|BindSequencerTime)
  (CallFunction|BindPlaySequence))

(fn SetManagerVariable
  (Variables|Manager|SetSequencerManager (Variables|/Game/Blueprint/Global/Manager/BP_SceneManager.BP_SceneManager_C|GetSequencerManager (Variables|Manager|GetScene%20Manager))))