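; Scene manager Blueprint that caches references to the game's other singleton managers and signals when initialization binding can run.
; Shortly after BeginPlay, it fetches and casts the Data, Investigation, Camera, Sequencer, UI and Desk managers into variables.
; A second, longer delay then fires the OnInitializationBind dispatcher, relying on timing rather than confirming that the references resolved.
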(event EventBeginPlay
  (Utilities|FlowControl|Sequence
    (:then_0
      (Utilities|FlowControl|Delay 0.2)
      (CallFunction|GetSingletonManager))
    (:then_1
      (Utilities|FlowControl|Delay 1.0)
      (Default|CallOnInitializationBind))))

(fn ConstructionScript)

(fn GetSingletonManager
  (Utilities|FlowControl|Sequence
    (:then_0
      (bind _asbp_data_manager (Utilities|Casting|CastToBP_DataManager (CallFunction|GetSingletonInstance "/Game/Blueprint/Global/Manager/BP_DataManager.BP_DataManager_C")))
      (Variables|Manager|SetDataManager _asbp_data_manager)
      (bind _asbp_investigation_manager (Utilities|Casting|CastToBP_InvestigationManager (CallFunction|GetSingletonInstance "/Game/Blueprint/Global/Manager/BP_InvestigationManager.BP_InvestigationManager_C")))
      (Variables|Manager|SetInvestigation%20Manager _asbp_investigation_manager))
    (:then_1
      (bind _asbp_camera_manager (Utilities|Casting|CastToBP_CameraManager (CallFunction|GetSingletonInstance "/Game/Blueprint/Global/Manager/BP_CameraManager.BP_CameraManager_C")))
      (Variables|Manager|SetCameraManager _asbp_camera_manager)
      (bind _asbp_sequencer_manager (Utilities|Casting|CastToBP_SequencerManager (CallFunction|GetSingletonInstance "/Game/Blueprint/Global/Manager/BP_SequencerManager.BP_SequencerManager_C")))
      (Variables|Manager|SetSequencerManager _asbp_sequencer_manager))
    (:then_2
      (bind _asbp_uimanager (Utilities|Casting|CastToBP_UIManager (CallFunction|GetSingletonInstance "/Game/Blueprint/Global/Manager/BP_UIManager.BP_UIManager_C")))
      (Variables|Manager|SetUIManager _asbp_uimanager)
      (bind _asbp_desk_manager (Utilities|Casting|CastToBP_DeskManager (CallFunction|GetSingletonInstance "/Game/Blueprint/Office/BP_DeskManager.BP_DeskManager_C")))
      (Variables|Desk|SetDesk%20Manager _asbp_desk_manager))))